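; BP_MuralElement is a configurable mural image actor whose texture, color and emissive level come from its own variables.
; The Construction Script creates a dynamic material instance from slot 0 of the MuralImage component, stores it in Material and feeds those variables into its parameters.
; Each placed element can therefore share a base material yet look different, with the result visible in the editor.
; The event graph holds no active logic.
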(event EventBeginPlay)

(event Collision|EventActorBeginOverlap
  (params (OtherActor :type Actor%20Object%20Reference)))

(event EventTick
  (params (DeltaSeconds :type Float%20%28single-precision%29)))

(fn ConstructionScript
  (bind _returnvalue (Rendering|Material|CreateDynamicMaterialInstance (Variables|Default|GetMuralImage) 0 (Rendering|Material|GetMaterial (Variables|Default|GetMuralImage) 0) "None" :!class /Script/Engine.PrimitiveComponent))
  (bind _output_get (Variables|Default|Setmaterial _returnvalue))
  (Rendering|Material|SetTextureParameterValue _output_get "Texture" (Variables|Default|Gettexture))
  (Rendering|Material|SetScalarParameterValue _output_get "Emissive" (Variables|Default|Getemissive) :!class /Script/Engine.MaterialInstanceDynamic)
  (Rendering|Material|SetVectorParameterValue _output_get "Color" (Variables|Default|GetColor) :!class /Script/Engine.MaterialInstanceDynamic))