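; BP_EnemyDetector is an overlap-based sensor that follows the player and reports nearby enemies to the companion.
; On BeginPlay it attaches to the player pawn, zeroes its relative location after a short delay, then caches the BP_Companion actor.
; Overlap events maintain an array of BP_Enemy_Master actors in range.
; Every tick it passes that array and a detected flag to the companion's EnemyDetection.
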(event EventBeginPlay
  ;[0.15 0.15 0.15 0.5] Attaching this actor to the players pawn
  (Transformation|AttachActorToActor (Game|Player|GetPlayerPawn 0) "None" "KeepRelative" "KeepRelative" "KeepRelative" true)
  (Utilities|FlowControl|Delay 0.2)
  (Transformation|SetActorRelativeLocation "0, 0, 0")
  (bind _returnvalue (Actor|GetActorOfClass "/Game/2D_Character/BP_Companion.BP_Companion_C"))
  (Variables|Default|SetCompanion _returnvalue))

(event EventTick
  (params (DeltaSeconds :type Float%20%28single-precision%29))
  ;[0.15 0.15 0.15 0.5] Checking for any enemies within the enemy detection range
  (Variables|Default|SetEnemyDetected (Utilities|Array|IsNotEmpty (Variables|Default|GetOverlapping%20Actors)))
  (Utilities|IsValid (Variables|Default|GetCompanion)
    (:Is%20Valid
      (Default|EnemyDetection (Variables|Default|GetCompanion) (Variables|Default|GetEnemyDetected) (Variables|Default|GetOverlapping%20Actors)))))

(event Collision|EventActorBeginOverlap
  (params (OtherActor :type Actor%20Object%20Reference))
  ;[0.15 0.15 0.15 0.5] Adding all enemies in range into an array
  (Class|KismetSystemLibrary|IsObjectOfSoftClass OtherActor "/Game/Enemies/BP_Enemy_Master.BP_Enemy_Master_C"
    (:True
      (Utilities|Array|Add (Variables|Default|GetOverlapping%20Actors) OtherActor))))

(event Collision|EventActorEndOverlap
  (params (OtherActor :type Actor%20Object%20Reference))
  ;[0.15 0.15 0.15 0.5] Removing out of range enemies
  (Utilities|Array|RemoveItem (Variables|Default|GetOverlapping%20Actors) OtherActor))

(fn ConstructionScript)