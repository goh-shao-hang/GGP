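; BP_Grapple is a grappling hook projectile that reports what it hits through event dispatchers.
; On BeginPlay it ignores the player pawn, caches the BP_2DCharacter, applies its Velocity and records its start location.
; A hit on the GameTraceChannel1 object type signals a landed hook, then stores the hooked location.
; Otherwise, BPI_GrappleableCreature actors get Grapple called and are reported as hooked, while anything else reports blocked.
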(event OnComponentHit(Sphere)
  (params (HitComponent :type Primitive%20Component%20Object%20Reference) (OtherActor :type Actor%20Object%20Reference) (OtherComp :type Primitive%20Component%20Object%20Reference) (NormalImpulse :type Vector :default "0, 0, 0") (Hit :type Hit%20Result%20Structure%20%28by%20ref%29))
  (Development|PrintString (Utilities|GetDisplayName OtherActor))
  (if (Utilities|Enum|Equal(Enum) (Collision|GetCollisionObjectType OtherComp) "ECC_GameTraceChannel1")
    (Default|CallOnHookLanded)
    (Variables|Default|SetHookedLocation (Transformation|GetWorldLocation (Variables|Default|GetSphere)))
    (else
      (bind _asbpi_grappleable_creature (Utilities|Casting|CastToBPI_GrappleableCreature OtherActor)
        (:then
          (Default|Grapple _asbpi_grappleable_creature)
          (Default|CallOnCreatureHooked _asbpi_grappleable_creature))
        (:CastFailed
          (Default|CallOnHookBlocked))))))

(event EventBeginPlay
  (Collision|IgnoreActorwhenMoving (Variables|Default|GetSphere) (Game|Player|GetPlayerPawn 0) true)
  (bind _asbp_2dcharacter (Utilities|Casting|CastToBP_2DCharacter (Game|Player|GetPlayerPawn 0)))
  (Variables|Default|SetAs%20BP%202DCharacter _asbp_2dcharacter)
  (Variables|/Script/Engine.MovementComponent|SetVelocity (Variables|Default|GetProjectileMovement) (Variables|Default|GetVelocity))
  (Variables|Default|SetStartLocation (Transformation|GetActorLocation)))

(fn ConstructionScript)