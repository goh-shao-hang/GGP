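; Side-scrolling spider enemy that activates when the player enters its detection volume, deals contact damage and dies at zero health.
; Tick sets facing and line-traces ahead, climbing walls via negative gravity, jumps and a rotated mesh.
; Overlap volumes trigger jumps and hits, while FollowPlayer, not called within this graph, chases or hops away based on PlayerHit.
; EnemyDamage, called by the companion, lowers health shown on camera-facing text.
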(event OnComponentBeginOverlap(PlayerDetection)
  (params (OverlappedComponent :type Primitive%20Component%20Object%20Reference) (OtherActor :type Actor%20Object%20Reference) (OtherComp :type Primitive%20Component%20Object%20Reference) (OtherBodyIndex :type Integer) (bFromSweep :type Boolean) (SweepResult :type Hit%20Result%20Structure%20%28by%20ref%29))
  ;[0.15 0.15 0.15 0.5] Enabling Movement When The Spider Is Detected
  (if (== OtherActor (Game|GetPlayerCharacter 0))
    (Variables|Default|SetplayerDetected true)))

(event OnComponentBeginOverlap(HitDetection)
  (params (OverlappedComponent :type Primitive%20Component%20Object%20Reference) (OtherActor :type Actor%20Object%20Reference) (OtherComp :type Primitive%20Component%20Object%20Reference) (OtherBodyIndex :type Integer) (bFromSweep :type Boolean) (SweepResult :type Hit%20Result%20Structure%20%28by%20ref%29))
  ;[0.15 0.15 0.15 0.5] Detecting when the enemy hits into the player
  (Utilities|IsValid OtherActor
    (:Is%20Valid
      (if (== OtherActor (Game|GetPlayerCharacter 0))
        (Development|PrintString "colliding into player")
        (Variables|Default|SetplayerHit true)
        (Variables|Default|SetDirection (not (Variables|Default|GetDirection)))
        (Game|Damage|ApplyDamage OtherActor (Variables|Default|GetattackDamage) 0 self)
        (Development|PrintString (Utilities|GetDisplayName OtherActor))))))

(event OnComponentBeginOverlap(JumpDetection)
  (params (OverlappedComponent :type Primitive%20Component%20Object%20Reference) (OtherActor :type Actor%20Object%20Reference) (OtherComp :type Primitive%20Component%20Object%20Reference) (OtherBodyIndex :type Integer) (bFromSweep :type Boolean) (SweepResult :type Hit%20Result%20Structure%20%28by%20ref%29))
  ;[0.15 0.15 0.15 0.5] Jumping when near the player
  (if (and (== OtherActor (Game|GetPlayerCharacter 0)) (not (Variables|Default|GethitWall)))
    (Character|Jump)))

(event Custom|Follow%20Player
  (bind _returnvalue (Game|GetPlayerCharacter 0))
  (bind _returnvalue_2 (Transformation|GetActorLocation))
  (bind _returnvalue_3 (Transformation|GetActorLocation _returnvalue))
  (bind _returnvalue_4 (Math|Vector|GetUnitDirection(Vector) _returnvalue_2 _returnvalue_3))
  ;[0.15 0.15 0.15 0.5] Following the player
  (if (Variables|Default|GetplayerDetected)
    (if (not (Variables|Default|GethitWall))
      (if (Variables|Default|GetplayerHit)
        (CallFunction|JumpingAwayfromPlayer)
        (else
          (Pawn|Input|AddMovementInput _returnvalue_4 1.0 false)
          ;[0.15 0.15 0.15 0.5] Changing the direction the enemy is facing
          (Variables|Default|SetDirection (>= (.X (Math|Vector|BreakVector _returnvalue_4)) 0.0)))))))

(event Custom|Jumping%20Away%20From%20Player
  ;[0.15 0.15 0.15 0.5] Jumping away from the player after they've been hit
  (Pawn|Input|AddMovementInput (Transformation|GetActorForwardVector) 1.0 true)
  (Utilities|FlowControl|Delay 0.2)
  (Character|Jump)
  (Utilities|FlowControl|Delay 0.5)
  (Variables|Default|SetplayerHit false))

(event EventTick
  (params (DeltaSeconds :type Float%20%28single-precision%29))
  (bind _spidermesh (Variables|Default|GetSpiderMesh))
  (bind _linetracestartpoint (Variables|Default|GetLineTraceStartPoint))
  (bind _returnvalue (Transformation|GetSocketLocation _linetracestartpoint "None"))
  (bind (_x _y _z) (Math|Vector|BreakVector _returnvalue))
  (Utilities|FlowControl|Sequence
    (:then_0
      (if (Variables|Default|GetplayerDetected)
        (Utilities|FlowControl|Sequence
          (:then_0
            ;[0.15 0.15 0.15 0.5] Rotating the enemy based on it's moving direction
            (if (Variables|Default|GetDirection)
              (Transformation|SetActorRotation "0, 0, 0")
              (else
                (Transformation|SetActorRotation "0.000000,180.000000,0.000000"))))
          (:then_1
            ;[0.15 0.15 0.15 0.5] Drawing line trace to detect walls
            (bind _outactors (Actor|GetAllActorswithInterface "/Game/Enemies/BPI_EnemyHealth.BPI_EnemyHealth_C"))
            (bind _returnvalue_2 (Collision|LineTraceByChannel _returnvalue (Math|Vector|MakeVector (Math|Float|SelectFloat (- _x 35.0) (+ _x 35.0) (Variables|Default|GetDirection)) _y _z) "TraceTypeQuery1" false _outactors "None"))
            (if _returnvalue_2
              ;[0.15 0.15 0.15 0.5] Climbing wall if wall was hit
              (Variables|Default|SetplayerHit false)
              (Variables|Default|SethitWall true)
              (Variables|/Script/Engine.CharacterMovementComponent|SetGravityScale (Variables|Character|GetCharacterMovement) -0.5)
              (Pawn|Input|AddMovementInput (Transformation|GetActorUpVector) 5.0 false)
              (Character|Jump)
              ;[0.15 0.15 0.15 0.5] Changing The Rotation Of The Spider's Mesh
              (Transformation|SetRelativeRotation _spidermesh "0.000000,-90.000000,-90.000000" false false)
              (else
                ;[0.15 0.15 0.15 0.5] Not climbing wall is wall wasn't hit
                (Variables|Default|SetplayerHit true)
                (Variables|Default|SethitWall false)
                (Variables|/Script/Engine.CharacterMovementComponent|SetGravityScale (Variables|Character|GetCharacterMovement) 1.0)
                (Transformation|SetRelativeRotation _spidermesh "0.000000,-90.000000,0.000000" false false)))))))
    (:then_1
      ;[0.15 0.15 0.15 0.5] Health Check
      (if (<= (Variables|Default|GetHealth) 0)
        ;[0.15 0.15 0.15 0.5] Enemy Death
        (Actor|DestroyActor)
        (else
          ;[0.15 0.15 0.15 0.5] Updating Health Text if enemy isn't dead
          (Rendering|Components|TextRender|SetText (Variables|Default|GetHealthText) (Utilities|Text|ToText(Integer) (Variables|Default|GetHealth)))
          ;[0.15 0.15 0.15 0.5] Rotating health text to face the camera
          (Transformation|SetWorldRotation (Variables|Default|GetHealthText) (Math|Rotator|MakeRotator 0.0 0.0 (.yaw (Math|Rotator|FindLookatRotation (Transformation|GetWorldLocation (Variables|Default|GetHealthText)) (Transformation|GetActorLocation (Game|GetPlayerCameraManager 0))))) false false))))))

(event EventEnemyDamage
  (params (Damage :type Integer))
  ;[0.15 0.15 0.15 0.5] Enemy damage. Called from the companion
  (Variables|Default|SetHealth (- (Variables|Default|GetHealth) Damage)))

(event EventBeginPlay
  (bind _returnvalue (Transformation|GetActorLocation))
  ;[0.15 0.15 0.15 0.5] Correcting position on the Y axis
  (Transformation|SetActorLocation (Math|Vector|MakeVector (.x _returnvalue) (.y (Transformation|GetActorLocation (Game|Player|GetPlayerPawn 0))) (.z _returnvalue)) false true))

(fn ConstructionScript)