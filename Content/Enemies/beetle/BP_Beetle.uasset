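; Flying beetle enemy for a 2D-plane game, cycling through attach, throw and dive attacks once the player enters its activation box.
; A Tick-driven state machine rises to a traced ceiling, tracks the player's X to drop a physics projectile, then dives to a traced floor point after a warning.
; Grapple pulls cancel attack timers, launching and stunning it under gravity before it reattaches.
; Companion damage flashes its dynamic material or destroys it.
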(event OnComponentBeginOverlap(ActivationBox)
  (params (OverlappedComponent :type Primitive%20Component%20Object%20Reference) (OtherActor :type Actor%20Object%20Reference) (OtherComp :type Primitive%20Component%20Object%20Reference) (OtherBodyIndex :type Integer) (bFromSweep :type Boolean) (SweepResult :type Hit%20Result%20Structure%20%28by%20ref%29))
  (Utilities|Casting|CastToBP_2DCharacter OtherActor)
  (CallFunction|OnAttach))

(event OnComponentBeginOverlap(Projectile)
  (params (OverlappedComponent :type Primitive%20Component%20Object%20Reference) (OtherActor :type Actor%20Object%20Reference) (OtherComp :type Primitive%20Component%20Object%20Reference) (OtherBodyIndex :type Integer) (bFromSweep :type Boolean) (SweepResult :type Hit%20Result%20Structure%20%28by%20ref%29))
  (if (Variables|Default|GetfinishedThrow)
    (if (not (== OtherActor self))
      (Variables|Default|SetfinishedThrow false)
      (CallFunction|EnableProjectile false)
      (bind _asbp_2dcharacter (Utilities|Casting|CastToBP_2DCharacter OtherActor))
      (Development|PrintString "HIT PLAYUER")
      (Game|Damage|ApplyDamage _asbp_2dcharacter (Variables|Default|GetprojectileDamage) 0 0))))

(event Custom|OnAttach
  (bind _returnvalue (Transformation|GetActorLocation))
  (Variables|Default|SetState "NewEnumerator0")
  (bind _outhit (Collision|LineTraceByChannel _returnvalue (+ _returnvalue (* (Math|Vector|VectorUp) 99999.0)) "TraceTypeQuery2" false 0 "ForOneFrame"))
  (bind _output_get (Variables|Default|SetpreattachLocation (Transformation|GetActorLocation)))
  (bind _lerp (Timeline|Timeline PlayFromStart)
    (:Update
      (Transformation|SetActorLocation (Math|Vector|Lerp(Vector) _output_get (- (.ImpactPoint (Collision|BreakHitResult _outhit)) "0.000000,0.000000,100.000000") _lerp) false false))
    (:Finished
      (CallFunction|OnThrow))))

(event Custom|OnDive
  (bind _returnvalue (Transformation|GetActorLocation))
  (bind _returnvalue_2 (+ _returnvalue "0.000000,0.000000,-1000.000000"))
  (Variables|Default|SetState "NewEnumerator2")
  (Niagara|SpawnSystematLocation "/Game/VFX/NS_Warning.NS_Warning" (Transformation|GetWorldLocation (Variables|Character|GetMesh)) "0, 0, 0" "1.000000,1.000000,1.000000" true true "AutoRelease")
  (bind _returnvalue_3 (Utilities|Time|SetTimerbyEvent (delegate Custom|PerformDiveAttack) 0.5))
  (Variables|Default|SetdiveTimer _returnvalue_3)
  (bind (_outhit _returnvalue_4) (Collision|LineTraceByChannel _returnvalue _returnvalue_2 "TraceTypeQuery2" false 0 "None"))
  (if _returnvalue_4
    (bind _output_get (Variables|Default|SetdiveTargetLoc (.ImpactPoint (Collision|BreakHitResult _outhit))))
    (Development|PrintString (Utilities|String|ToString(Vector) _output_get))
    (else
      (bind _output_get_2 (Variables|Default|SetdiveTargetLoc _returnvalue_2))
      (Development|PrintString (Utilities|String|ToString(Vector) _output_get_2)))))

(event Custom|OnStunned
  (Variables|/Script/Engine.CharacterMovementComponent|SetGravityScale (Variables|Character|GetCharacterMovement) 1.0)
  (Variables|Default|SetState "NewEnumerator3")
  (Utilities|Time|SetTimerbyEvent (delegate Custom|OnStunEnd) (Variables|Default|GetstunDuration)))

(event Custom|OnStunEnd
  (Variables|/Script/Engine.CharacterMovementComponent|SetGravityScale (Variables|Character|GetCharacterMovement) 0.0)
  (CallFunction|OnAttach))

(event Custom|OnThrow
  (Variables|Default|SetState "NewEnumerator1")
  (Variables|Default|SetfinishedThrow false))

(event Custom|UpdateThrow
  (params (deltaTime :type Float%20%28double-precision%29))
  (bind _returnvalue (Transformation|GetActorLocation))
  (bind _returnvalue_2 (Transformation|GetActorLocation))
  (bind _projectile (Variables|Default|GetProjectile))
  (bind (_x _y _z) (Math|Vector|BreakVector _returnvalue_2))
  (Transformation|SetActorLocation (Math|Interpolation|VInterpTo _returnvalue_2 (Math|Vector|MakeVector (.x (Transformation|GetActorLocation (Game|GetPlayerCharacter 0))) _y _z) deltaTime (Variables|Default|GetfollowSpeed)) true false)
  (if (not (Variables|Default|GetfinishedThrow))
    (bind _outhit (Class|KismetSystemLibrary|SphereTraceSinglebyProfile _returnvalue (- _returnvalue "0.000000,0.000000,1000.000000") 5e+01 "Pawn" false 0 "ForOneFrame" true))
    (Utilities|Casting|CastToBP_2DCharacter (.HitActor (Collision|BreakHitResult _outhit)))
    (Physics|SetPhysicsLinearVelocity _projectile "0, 0, 0" false "None")
    (Physics|SetSimulatePhysics _projectile true)
    (bind _returnvalue_3 (Utilities|Time|SetTimerbyEvent (EventDispatchers|CreateEvent :!event Custom|OnDive) 2.0))
    (Variables|Default|SetthrowToDiveTimer _returnvalue_3)
    (Variables|Default|SetfinishedThrow true)))

(event Custom|Flash
  (bind _value (Timeline|TM_Flash PlayFromStart)
    (:Update
      (Rendering|Material|SetScalarParameterValue (Variables|Default|Getmaterial) "Flash" (* _value 1.0) :!class /Script/Engine.MaterialInstanceDynamic))))

(event Custom|PerformDiveAttack
  (Variables|Default|Setdiving true))

(event Custom|UpdateDiving
  (params (deltaTime :type Float%20%28double-precision%29))
  (bind _returnvalue (Transformation|GetActorLocation))
  (bind _divespeed (Variables|Default|GetdiveSpeed))
  (bind _divetargetloc (Variables|Default|GetdiveTargetLoc))
  (bind _returnvalue_2 (Math|Interpolation|VInterptoConstant _returnvalue _divetargetloc deltaTime _divespeed))
  (if (Variables|Default|Getdiving)
    (Transformation|SetActorLocation _returnvalue_2 false false)
    (if (Utilities|Operators|EqualEqual _returnvalue_2 _divetargetloc 1e+01)
      (Variables|Default|Setdiving false)
      (Utilities|FlowControl|Delay 1.0)
      (CallFunction|OnAttach)
      (Variables|Default|SetfinishedThrow false)
      (CallFunction|EnableProjectile true))))

(event Custom|UpdateAttach
  (params (deltaTime :type Float%20%28double-precision%29)))

(event EventGrapple
  ;[0.15 0.15 0.15 0.5] Grappled Reaction
  (Variables|Default|Setgrappled true)
  (bind _returnvalue (Utilities|Time|SetTimerbyEvent (delegate EventBreakFreefromGrapple) 3.0))
  (Variables|Default|SetGrappledTimer _returnvalue))

(event EventPulledReaction
  (bind _returnvalue (Transformation|GetActorLocation))
  (bind _returnvalue_2 (Game|GetPlayerCharacter 0))
  (bind _launchforce (Variables|Default|GetlaunchForce))
  (bind _returnvalue_3 (Transformation|GetActorLocation _returnvalue_2))
  (bind _returnvalue_4 (- _returnvalue_3 _returnvalue))
  (bind _returnvalue_5 (Math|Vector|Normalize _returnvalue_4))
  (bind _returnvalue_6 (* _returnvalue_5 _launchforce))
  ;[0.15 0.15 0.15 0.5] Grappled Reaction
  (Utilities|Time|ClearandInvalidateTimerbyHandle (Variables|Default|GetGrappledTimer))
  (Utilities|Time|ClearandInvalidateTimerbyHandle (Variables|Default|GetthrowToDiveTimer))
  (Utilities|Time|ClearandInvalidateTimerbyHandle (Variables|Default|GetdiveTimer))
  (Character|LaunchCharacter (Math|Vector|MakeVector (.x _returnvalue_6) 0.0 (+ (.z _returnvalue_6) 2.5e+02)) true true)
  (Variables|Default|Setgrappled false)
  (CallFunction|OnStunned))

(event EventTick
  (params (DeltaSeconds :type Float%20%28single-precision%29))
  (switch Utilities|FlowControl|Switch|SwitchonE_BeetleState (Variables|Default|GetState)
    (:NewEnumerator0
      (CallFunction|UpdateAttach DeltaSeconds))
    (:NewEnumerator1
      (CallFunction|UpdateThrow DeltaSeconds))
    (:NewEnumerator2
      (CallFunction|UpdateDiving DeltaSeconds))))

(event EventBreakFreefromGrapple
  ;[0.15 0.15 0.15 0.5] Grappled Reaction
  (Variables|Default|Setgrappled false)
  (bind _asbp_2dcharacter (Utilities|Casting|CastToBP_2DCharacter (Game|GetPlayerCharacter 0)))
  (Default|RetractGrapple _asbp_2dcharacter))

(event EventEnemyDamage
  (params (Damage :type Integer))
  ;[0.15 0.15 0.15 0.5] Enemy damage. Called from the companion
  (Variables|Default|SetHealth (- (Variables|Default|GetHealth) Damage))
  ;[0.15 0.15 0.15 0.5] Health Check
  (if (<= (Variables|Default|GetHealth) 0)
    ;[0.15 0.15 0.15 0.5] Enemy Death
    (Actor|DestroyActor)
    (else
      (CallFunction|Flash))))

(event EventBeginPlay
  (bind _returnvalue (Transformation|GetActorLocation))
  (bind _staticmesh (Variables|Default|GetStaticMesh))
  (bind _projectile (Variables|Default|GetProjectile))
  ;[0.15 0.15 0.15 0.5] Correcting position on the Y axis
  (Transformation|SetActorLocation (Math|Vector|MakeVector (.x _returnvalue) (.y (Transformation|GetActorLocation (Game|Player|GetPlayerPawn 0))) (.z _returnvalue)) false true)
  (Collision|IgnoreActorwhenMoving _projectile (Components|GetOwner _projectile) true)
  (bind _returnvalue_2 (Rendering|Material|CreateDynamicMaterialInstance _staticmesh 0 (Rendering|Material|GetMaterial _staticmesh 0) "None" :!class /Script/Engine.PrimitiveComponent))
  (Variables|Default|Setmaterial _returnvalue_2))

(event Collision|EventActorBeginOverlap
  (params (OtherActor :type Actor%20Object%20Reference)))

(fn ConstructionScript)

(fn EnableProjectile
  (params (enabled? :type Boolean))
  (bind _projectile (Variables|Default|GetProjectile))
  (Rendering|SetVisibility _projectile enabled? false)
  (Components|Tick|SetComponentTickEnabled _projectile enabled?)
  (if enabled?
    (Collision|SetCollisionEnabled _projectile "QueryAndPhysics")
    (Transformation|AttachComponentToComponent (Variables|Default|GetProjectile) (Variables|Character|GetMesh) "None" "KeepRelative" "KeepRelative" "KeepRelative" true)
    (Transformation|SetRelativeLocation (Variables|Default|GetProjectile) "50.000000,0.000000,-45.000000" false true)
    (else
      (Collision|SetCollisionEnabled _projectile "NoCollision")))
  (Physics|SetSimulatePhysics (Variables|Default|GetProjectile) false))