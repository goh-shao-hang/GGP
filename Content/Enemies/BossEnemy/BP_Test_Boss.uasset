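; Test spider boss for a side-view game that aligns to the player's Y and runs a Follow, Attack, Strafe and Stunned state machine on Tick.
; Following uses line traces to stop at cliffs and climb walls, then telegraphs a timed pounce that leads into strafing.
; AnimBP dispatchers open a hit-once damage window during attacks.
; Grapple pulls launch and stun it, while damage updates health text, flashes materials or destroys it.
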(event OnComponentBeginOverlap(PlayerDetection)
  (params (OverlappedComponent :type Primitive%20Component%20Object%20Reference) (OtherActor :type Actor%20Object%20Reference) (OtherComp :type Primitive%20Component%20Object%20Reference) (OtherBodyIndex :type Integer) (bFromSweep :type Boolean) (SweepResult :type Hit%20Result%20Structure%20%28by%20ref%29))
  ;[0.15 0.15 0.15 0.5] Enabling Movement When The Spider Is Detected
  (if (== OtherActor (Game|GetPlayerCharacter 0))
    (Variables|Default|SetplayerDetected true)))

(event OnComponentBeginOverlap(HitDetection)
  (params (OverlappedComponent :type Primitive%20Component%20Object%20Reference) (OtherActor :type Actor%20Object%20Reference) (OtherComp :type Primitive%20Component%20Object%20Reference) (OtherBodyIndex :type Integer) (bFromSweep :type Boolean) (SweepResult :type Hit%20Result%20Structure%20%28by%20ref%29)))

(event OnComponentBeginOverlap(JumpDetection)
  (params (OverlappedComponent :type Primitive%20Component%20Object%20Reference) (OtherActor :type Actor%20Object%20Reference) (OtherComp :type Primitive%20Component%20Object%20Reference) (OtherBodyIndex :type Integer) (bFromSweep :type Boolean) (SweepResult :type Hit%20Result%20Structure%20%28by%20ref%29)))

(event Custom|Strafe
  (bind _returnvalue (Game|GetPlayerCharacter 0))
  (bind _returnvalue_2 (Transformation|GetActorLocation))
  (bind _returnvalue_3 (Transformation|GetActorLocation _returnvalue))
  (bind _returnvalue_4 (Math|Vector|GetUnitDirection(Vector) _returnvalue_2 _returnvalue_3))
  ;[0.15 0.15 0.15 0.5] Strafe
  (if (Variables|Default|GetplayerDetected)
    (if (not (Variables|Default|GethitWall))
      (bind _cliffhit (CallFunction|CheckforCliffs))
      (if _cliffhit
        (Pawn|Input|AddMovementInput _returnvalue_4 (Math|Float|SelectFloat 1.0 -1.0 (>= (Math|Vector|Distance(Vector) _returnvalue_2 _returnvalue_3) (Variables|Default|GetstrafeDistance))) false)
        ;[0.15 0.15 0.15 0.5] Changing the direction the enemy is facing
        (bind _output_get (Variables|Default|SetDirection (>= (.X (Math|Vector|BreakVector _returnvalue_4)) 0.0)))
        (CallFunction|FnUpdateFacing)))))

(event Custom|PrepareAttack
  (Niagara|SpawnSystematLocation "/Game/VFX/NS_Warning.NS_Warning" (Transformation|GetWorldLocation (Variables|Default|GetHitDetection)) "0, 0, 0" "1.000000,1.000000,1.000000" true true "AutoRelease")
  (Variables|Default|SetState "NewEnumerator1")
  (bind _returnvalue (Utilities|Time|SetTimerbyEvent (delegate Custom|Pounce) (Variables|Default|GetattackPrepareTime)))
  (Variables|Default|SetattackPrepareTimer _returnvalue)
  (Variables|/Game/Enemies/BossEnemy/SpiderBoss_AnimBlueprint.SpiderBoss_AnimBlueprint_C|SetAttacking (Variables|Default|GetanimBP) false)
  (Animation|Montage|PlayMontage (Variables|Character|GetMesh) "/Game/Enemies/SpiderAnimations/JumpAnimation/Montage_Anticipate.Montage_Anticipate" 0.2 0.0 "None" false))

(event Custom|OnStunned
  (bind _animbp (Variables|Default|GetanimBP))
  (Variables|Default|SetState "NewEnumerator3")
  (Variables|/Game/Enemies/BossEnemy/SpiderBoss_AnimBlueprint.SpiderBoss_AnimBlueprint_C|SetStunned _animbp false)
  (Variables|/Game/Enemies/BossEnemy/SpiderBoss_AnimBlueprint.SpiderBoss_AnimBlueprint_C|SetAttacking _animbp false)
  (Utilities|Time|SetTimerbyEvent (delegate Custom|OnStunEnd) (Variables|Default|GetstunDuration))
  (Utilities|Time|ClearandInvalidateTimerbyHandle (Variables|Default|GetRetreatTimer))
  (Utilities|Time|ClearandInvalidateTimerbyHandle (Variables|Default|GetattackPrepareTimer)))

(event Custom|OnFollow
  (Variables|/Script/Engine.CharacterMovementComponent|SetMaxWalkSpeed (Variables|Character|GetCharacterMovement) (Variables|Default|GetfollowSpeed))
  (Variables|Default|SetState "NewEnumerator0"))

(event Custom|OnStrafe
  (Variables|/Script/Engine.CharacterMovementComponent|SetMaxWalkSpeed (Variables|Character|GetCharacterMovement) (Variables|Default|GetstrafeSpeed))
  (Variables|Default|SetState "NewEnumerator2"))

(event Custom|OnStunEnd
  (Variables|/Game/Enemies/BossEnemy/SpiderBoss_AnimBlueprint.SpiderBoss_AnimBlueprint_C|SetStunned (Variables|Default|GetanimBP) false)
  (CallFunction|OnFollow))

(event Custom|ActivateHitbox
  (Variables|Default|SethitboxActivated true)
  (Utilities|Array|Clear (Variables|Default|GettargetsHit)))

(event Custom|DeactivateHitbox
  (Variables|Default|SethitboxActivated false))

(event Custom|CheckHitboxOverlap
  ;[0.15 0.15 0.15 0.5] Detecting when the enemy hits into the player
  (if (Variables|Default|GethitboxActivated)
    (bind _asbp_2dcharacter (Utilities|Casting|CastToBP_2DCharacter (Utilities|Array|Get(acopy) (Collision|GetOverlappingActors (Variables|Default|GetHitDetection) "/Game/2D_Character/BP_2DCharacter.BP_2DCharacter_C" :!class /Script/Engine.PrimitiveComponent))))
    (if (not (Utilities|Array|ContainsItem (Variables|Default|GettargetsHit) _asbp_2dcharacter))
      (Variables|Default|SetplayerHit true)
      (Game|Damage|ApplyDamage 0 (Variables|Default|GetattackDamage) 0 self)
      (Utilities|Array|Add (Variables|Default|GettargetsHit) _asbp_2dcharacter))))

(event Custom|Pounce
  (bind _launchvelocity (Variables|Default|GetlaunchVelocity))
  (Character|LaunchCharacter (Math|Vector|MakeVector (* (Math|Float|SelectFloat 1.0 -1.0 (Variables|Default|GetDirection)) (.x _launchvelocity)) (.y _launchvelocity) (.z _launchvelocity)) true true)
  (Animation|Montage|PlayMontage (Variables|Character|GetMesh) "/Game/Enemies/SpiderAnimations/JumpAnimation/Montage_Jump.Montage_Jump" 2.0 0.0 "None" false
    (:OnCompleted
      (Variables|/Game/Enemies/BossEnemy/SpiderBoss_AnimBlueprint.SpiderBoss_AnimBlueprint_C|SetAttacking (Variables|Default|GetanimBP) false)
      (CallFunction|OnStrafe)
      (bind _returnvalue (Utilities|Time|SetTimerbyEvent (EventDispatchers|CreateEvent :!event Custom|OnFollow) 1.5))
      (Variables|Default|SetRetreatTimer _returnvalue)
      (Variables|/Script/Engine.CharacterMovementComponent|SetMaxWalkSpeed (Variables|Character|GetCharacterMovement) (Variables|Default|GetstrafeSpeed)))))

(event Custom|CheckAttackRange
  ;[0.15 0.15 0.15 0.5] Attack Detection
  (Utilities|Casting|CastToBP_2DCharacter (Utilities|Array|Get(acopy) (Collision|GetOverlappingActors (Variables|Default|GetJumpDetection) "/Game/2D_Character/BP_2DCharacter.BP_2DCharacter_C" :!class /Script/Engine.PrimitiveComponent)))
  (bind _walldetected (CallFunction|CheckforWall (Variables|Default|GetDirection)))
  (if (not _walldetected)
    (CallFunction|PrepareAttack)))

(event Custom|Flash
  (bind _value (Timeline|Timeline PlayFromStart)
    (:Update
      (for _array_element (Variables|Default|GetMaterials)
        (Rendering|Material|SetScalarParameterValue _array_element "Flash" (* _value 2.0) :!class /Script/Engine.MaterialInstanceDynamic)))))

(event Custom|Follow%20Player
  (bind _returnvalue (Game|GetPlayerCharacter 0))
  (bind _returnvalue_2 (Transformation|GetActorLocation))
  (bind _mesh (Variables|Character|GetMesh))
  (bind _returnvalue_3 (Transformation|GetActorLocation _returnvalue))
  (bind _returnvalue_4 (Math|Vector|GetUnitDirection(Vector) _returnvalue_2 _returnvalue_3))
  ;[0.15 0.15 0.15 0.5] Following the player
  (if (Variables|Default|GetplayerDetected)
    (if (not (Variables|Default|GethitWall))
      (bind _cliffhit (CallFunction|CheckforCliffs))
      (if _cliffhit
        (Pawn|Input|AddMovementInput _returnvalue_4 1.0 false)
        (else
          (Variables|/Script/Engine.MovementComponent|SetVelocity (Variables|Character|GetCharacterMovement) "0, 0, 0")))
      ;[0.15 0.15 0.15 0.5] Changing the direction the enemy is facing
      (bind _output_get (Variables|Default|SetDirection (>= (.X (Math|Vector|BreakVector _returnvalue_4)) 0.0)))
      (CallFunction|FnUpdateFacing)
      (bind _walldetected (CallFunction|CheckforWall _output_get))
      (Physics|SetEnableGravity (Variables|Collision|GetCapsuleComponent) _walldetected)
      (if _walldetected
        (Character|LaunchCharacter (Math|Vector|MakeVector 0.0 0.0 (Variables|Default|GetfollowSpeed)) false true)
        (Transformation|SetRelativeRotation _mesh "0.000000,0.000000,-90.000000" false false)
        (else
          (Transformation|SetRelativeRotation _mesh "0, 0, 0" false false))))))

(event EventGrapple
  ;[0.15 0.15 0.15 0.5] Grappled Reaction
  (Variables|Default|Setgrappled true)
  (bind _returnvalue (Utilities|Time|SetTimerbyEvent (delegate EventBreakFreefromGrapple) 3.0))
  (Variables|Default|SetGrappledTimer _returnvalue))

(event EventPulledReaction
  (bind _returnvalue (Transformation|GetActorLocation))
  (bind _returnvalue_2 (Game|GetPlayerCharacter 0))
  (bind _launchforce (Variables|Default|GetlaunchForce))
  (bind _returnvalue_3 (Transformation|GetActorLocation _returnvalue_2))
  (bind _returnvalue_4 (- _returnvalue_3 _returnvalue))
  (bind _returnvalue_5 (Math|Vector|Normalize _returnvalue_4))
  (bind _returnvalue_6 (* _returnvalue_5 _launchforce))
  ;[0.15 0.15 0.15 0.5] Grappled Reaction
  (Utilities|Time|ClearandInvalidateTimerbyHandle (Variables|Default|GetGrappledTimer))
  (Utilities|Time|ClearandInvalidateTimerbyHandle (Variables|Default|GetattackPrepareTimer))
  (Character|LaunchCharacter (Math|Vector|MakeVector (.x _returnvalue_6) 0.0 (+ (.z _returnvalue_6) 2.5e+02)) true true)
  (Variables|Default|Setgrappled false)
  (CallFunction|OnStunned))

(event EventTick
  (params (DeltaSeconds :type Float%20%28single-precision%29))
  (switch Utilities|FlowControl|Switch|SwitchonE_SpiderState (Variables|Default|GetState)
    (:NewEnumerator0
      (CallFunction|FollowPlayer)
      (CallFunction|CheckAttackRange))
    (:NewEnumerator1
      (CallFunction|CheckHitboxOverlap))
    (:NewEnumerator2
      (CallFunction|Strafe))))

(event EventBreakFreefromGrapple
  ;[0.15 0.15 0.15 0.5] Grappled Reaction
  (Variables|Default|Setgrappled false)
  (bind _asbp_2dcharacter (Utilities|Casting|CastToBP_2DCharacter (Game|GetPlayerCharacter 0)))
  (Default|RetractGrapple _asbp_2dcharacter))

(event EventEnemyDamage
  (params (Damage :type Integer))
  ;[0.15 0.15 0.15 0.5] Enemy damage. Called from the companion
  (Development|PrintString "HIT")
  (Variables|Default|SetHealth (- (Variables|Default|GetHealth) Damage))
  ;[0.15 0.15 0.15 0.5] Health Check
  (if (<= (Variables|Default|GetHealth) 0)
    ;[0.15 0.15 0.15 0.5] Enemy Death
    (Actor|DestroyActor)
    (else
      ;[0.15 0.15 0.15 0.5] Updating Health Text if enemy isn't dead
      (Rendering|Components|TextRender|SetText (Variables|Default|GetHealthText) (Utilities|Text|ToText(Integer) (Variables|Default|GetHealth)))
      (CallFunction|Flash))))

(event EventBeginPlay
  (bind _returnvalue (Transformation|GetActorLocation))
  (bind _mesh (Variables|Character|GetMesh))
  ;[0.15 0.15 0.15 0.5] Correcting position on the Y axis
  (Transformation|SetActorLocation (Math|Vector|MakeVector (.x _returnvalue) (.y (Transformation|GetActorLocation (Game|Player|GetPlayerPawn 0))) (.z _returnvalue)) false true)
  (CallFunction|OnFollow)
  (Utilities|FlowControl|Sequence
    (:then_0
      (for (_array_element _array_index) (Rendering|Material|GetMaterials _mesh)
        (bind _returnvalue_2 (Rendering|Material|CreateDynamicMaterialInstance _mesh _array_index _array_element "None" :!class /Script/Engine.PrimitiveComponent))
        (Utilities|Array|Add (Variables|Default|GetMaterials) _returnvalue_2)))
    (:then_1
      (bind _asspider_boss_anim_blueprint (Utilities|Casting|CastToSpiderBoss_AnimBlueprint (Components|SkeletalMesh|GetAnimInstance (Variables|Character|GetMesh))))
      (bind _output_get (Variables|Default|SetanimBP _asspider_boss_anim_blueprint))
      (EventDispatchers|BindEventtoOnActivateHitbox _output_get (delegate Custom|ActivateHitbox))
      (EventDispatchers|BindEventtoOnDeactivateHitbox _output_get (delegate Custom|DeactivateHitbox)))))

(fn ConstructionScript)

(fn FnUpdateFacing
  (if (Variables|Default|GetDirection)
    (Transformation|SetActorRotation "0.000000,-90.000000,0.000000")
    (else
      (Transformation|SetActorRotation "0.000000,90.000000,0.000000"))))

(fn CheckforWall
  (params (facingRight :type Boolean))
  (bind _linetracestartpoint (Variables|Default|GetLineTraceStartPoint))
  (bind _returnvalue (Transformation|GetWorldLocation _linetracestartpoint))
  (bind (_x _y _z) (Math|Vector|BreakVector _returnvalue))
  (bind _returnvalue_2 (Collision|LineTraceByChannel _returnvalue (Math|Vector|MakeVector (+ (* (Variables|Default|GetwallCheckDistance) (Math|Float|SelectFloat 1.0 -1.0 facingRight)) _x) _y _z) "TraceTypeQuery2" false (Utilities|Array|MakeArray (Game|GetPlayerCharacter 0)) "ForOneFrame"))
  (return _returnvalue_2))

(fn CheckforCliffs
  (bind _cliffcheck (Variables|Default|GetCliffCheck))
  (bind _returnvalue (Transformation|GetWorldLocation _cliffcheck))
  (bind (_outhit _returnvalue_2) (Collision|LineTraceByChannel _returnvalue (+ _returnvalue (* (Math|Vector|VectorDown) (Variables|Default|GetcliffCheckLength))) "TraceTypeQuery2" false 0 "ForOneFrame"))
  (return (.bBlockingHit (Collision|BreakHitResult _outhit))))