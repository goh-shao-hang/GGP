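; Chasing spider boss for the 2D character that kills the player on contact, aligned to the player's Y position at BeginPlay.
; Entering its chase trigger starts a timeline drop on Z, after which Tick moves it at constant speed along X toward a fixed end point.
; While chasing, it polls its hitbox each tick and applies lethal damage.
; The player's respawn event returns it to its start, ready to retrigger.
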(event OnComponentBeginOverlap(chaseTrigger)
  (params (OverlappedComponent :type Primitive%20Component%20Object%20Reference) (OtherActor :type Actor%20Object%20Reference) (OtherComp :type Primitive%20Component%20Object%20Reference) (OtherBodyIndex :type Integer) (bFromSweep :type Boolean) (SweepResult :type Hit%20Result%20Structure%20%28by%20ref%29))
  (if (not (Variables|Default|Getactivated))
    (Utilities|Casting|CastToBP_2DCharacter OtherActor)
    (CallFunction|Activate)))

(event OnComponentBeginOverlap(HitDetection)
  (params (OverlappedComponent :type Primitive%20Component%20Object%20Reference) (OtherActor :type Actor%20Object%20Reference) (OtherComp :type Primitive%20Component%20Object%20Reference) (OtherBodyIndex :type Integer) (bFromSweep :type Boolean) (SweepResult :type Hit%20Result%20Structure%20%28by%20ref%29)))

(event Custom|ResetChase
  (CallFunction|StopChase)
  (Transformation|SetActorLocation (Variables|Default|GetoriginalLocation) false true)
  (Variables|Default|Setactivated false)
  (Variables|Default|SetisChasing false))

(event Custom|StopChase
  (bind _returnvalue (Transformation|GetActorLocation))
  (bind _lerp (Timeline|TM_DropIn Stop)
    (:Update
      (Transformation|SetActorLocation (Math|Vector|MakeVector (.x _returnvalue) (.y _returnvalue) (Math|Float|Lerp (Variables|Default|GetstartZ) (Variables|Default|GetendZ) _lerp)) false false))
    (:Finished
      (Variables|Default|SetisChasing true))))

(event Custom|CheckHitboxOverlap
  ;[0.15 0.15 0.15 0.5] Detecting when the enemy hits into the player
  (if true
    (bind _asbp_2dcharacter (Utilities|Casting|CastToBP_2DCharacter (Utilities|Array|Get(acopy) (Collision|GetOverlappingActors (Variables|Default|GetHitDetection) "/Game/2D_Character/BP_2DCharacter.BP_2DCharacter_C" :!class /Script/Engine.PrimitiveComponent))))
    (Development|PrintString "colliding into player")
    (Variables|Default|SetplayerHit true)
    (Game|Damage|ApplyDamage _asbp_2dcharacter 999.0 0 self)
    (Development|PrintString "Killed player")))

(event Custom|Activate
  (bind _returnvalue (Transformation|GetActorLocation))
  (Variables|Default|Setactivated true)
  (bind _lerp (Timeline|TM_DropIn PlayFromStart)
    (:Update
      (Transformation|SetActorLocation (Math|Vector|MakeVector (.x _returnvalue) (.y _returnvalue) (Math|Float|Lerp (Variables|Default|GetstartZ) (Variables|Default|GetendZ) _lerp)) false false))
    (:Finished
      (Variables|Default|SetisChasing true))))

(event EventTick
  (params (DeltaSeconds :type Float%20%28single-precision%29))
  (bind _returnvalue (Transformation|GetActorLocation))
  (if (Variables|Default|GetisChasing)
    (Transformation|SetActorLocation (Math|Vector|MakeVector (Math|Interpolation|FInterptoConstant (.x _returnvalue) (Variables|Default|GetendX) DeltaSeconds (Variables|Default|Getspeed)) (.y _returnvalue) (.z _returnvalue)) false true)
    (CallFunction|CheckHitboxOverlap)))

(event EventBeginPlay
  ;[0.15 0.15 0.15 0.5] Correcting position on the Y axis
  (Transformation|SetActorLocation (Math|Vector|MakeVector (Variables|Default|GetstartX) (.y (Transformation|GetActorLocation (Game|Player|GetPlayerPawn 0))) (Variables|Default|GetstartZ)) false true)
  (Variables|Default|SetoriginalLocation (Transformation|GetActorLocation))
  (Utilities|FlowControl|Sequence
    (:then_0
      (bind _asspider_boss_anim_blueprint (Utilities|Casting|CastToSpiderBoss_AnimBlueprint (Components|SkeletalMesh|GetAnimInstance (Variables|Character|GetMesh))))
      (Variables|Default|SetanimBP _asspider_boss_anim_blueprint))
    (:then_1
      (bind _asbp_2dcharacter (Utilities|Casting|CastToBP_2DCharacter (Game|GetPlayerCharacter 0)))
      (EventDispatchers|BindEventtoOnRespawned _asbp_2dcharacter (delegate Custom|ResetChase)))))

(fn ConstructionScript)