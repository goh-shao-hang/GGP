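; Side-scrolling spider enemy that detects the player, climbs walls and deals contact damage, snapped to the player's Y plane at BeginPlay.
; Tick traces ahead for walls, climbing with negative gravity and Jump and reversing under ceilings.
; FollowPlayer steers toward the player, and a proximity overlap triggers jumps.
; EnemyDamage updates health text or destroys it; grapples break after three seconds, while pulls launch it playerward and briefly stun it.
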(event OnComponentBeginOverlap(PlayerDetection)
  (params (OverlappedComponent :type Primitive%20Component%20Object%20Reference) (OtherActor :type Actor%20Object%20Reference) (OtherComp :type Primitive%20Component%20Object%20Reference) (OtherBodyIndex :type Integer) (bFromSweep :type Boolean) (SweepResult :type Hit%20Result%20Structure%20%28by%20ref%29))
  ;[0.15 0.15 0.15 0.5] Enabling Movement When The Spider Is Detected
  (if (== OtherActor (Game|GetPlayerCharacter 0))
    (Variables|Default|SetplayerDetected true)))

(event OnComponentBeginOverlap(HitDetection)
  (params (OverlappedComponent :type Primitive%20Component%20Object%20Reference) (OtherActor :type Actor%20Object%20Reference) (OtherComp :type Primitive%20Component%20Object%20Reference) (OtherBodyIndex :type Integer) (bFromSweep :type Boolean) (SweepResult :type Hit%20Result%20Structure%20%28by%20ref%29))
  ;[0.15 0.15 0.15 0.5] Detecting when the enemy hits into the player
  (Utilities|IsValid OtherActor
    (:Is%20Valid
      (if (== OtherActor (Game|GetPlayerCharacter 0))
        (Development|PrintString "colliding into player")
        (Variables|Default|SetplayerHit true)
        ;;[0.15 0.15 0.15 0.5] Seems redundant?
        (Variables|Default|SetDirection (not (Variables|Default|GetDirection)))
        (Game|Damage|ApplyDamage OtherActor (Variables|Default|GetattackDamage) 0 self)
        (Development|PrintString (Utilities|GetDisplayName OtherActor))))))

(event OnComponentBeginOverlap(JumpDetection)
  (params (OverlappedComponent :type Primitive%20Component%20Object%20Reference) (OtherActor :type Actor%20Object%20Reference) (OtherComp :type Primitive%20Component%20Object%20Reference) (OtherBodyIndex :type Integer) (bFromSweep :type Boolean) (SweepResult :type Hit%20Result%20Structure%20%28by%20ref%29))
  ;[0.15 0.15 0.15 0.5] Jumping when near the player
  (if (and (== OtherActor (Game|GetPlayerCharacter 0)) (not (Variables|Default|GethitWall)))
    (Character|Jump)))

(event Custom|Follow%20Player
  (bind _returnvalue (Game|GetPlayerCharacter 0))
  (bind _returnvalue_2 (Transformation|GetActorLocation))
  (bind _returnvalue_3 (Transformation|GetActorLocation _returnvalue))
  (bind _returnvalue_4 (Math|Vector|GetUnitDirection(Vector) _returnvalue_2 _returnvalue_3))
  ;[0.15 0.15 0.15 0.5] Following the player
  (if (not (Variables|Default|GetStunned))
    (if (Variables|Default|GetplayerDetected)
      (if (not (Variables|Default|GethitWall))
        (if (Variables|Default|GetplayerHit)
          _
          (else
            _))
        (Pawn|Input|AddMovementInput _returnvalue_4 1.0 false)
        ;;[0.15 0.15 0.15 0.5] Changing the direction the enemy is facing
        (Variables|Default|SetDirection (>= (.X (Math|Vector|BreakVector _returnvalue_4)) 0.0))))))

(event Custom|Jumping%20Away%20From%20Player
  ;[0.15 0.15 0.15 0.5] Jumping away from the player after they've been hit
)

(event EventGrapple
  ;[0.15 0.15 0.15 0.5] Grappled Reaction
  (Variables|Default|Setgrappled true)
  (bind _returnvalue (Utilities|Time|SetTimerbyEvent (delegate EventBreakFreefromGrapple) 3.0))
  (Variables|Default|SetGrappledTimer _returnvalue))

(event EventPulledReaction
  (bind _returnvalue (Transformation|GetActorLocation))
  (bind _returnvalue_2 (Game|GetPlayerCharacter 0))
  (bind _launchforce (Variables|Default|GetlaunchForce))
  (bind _returnvalue_3 (Transformation|GetActorLocation _returnvalue_2))
  (bind _returnvalue_4 (- _returnvalue_3 _returnvalue))
  (bind _returnvalue_5 (Math|Vector|Normalize _returnvalue_4))
  (bind _returnvalue_6 (* _returnvalue_5 _launchforce))
  ;[0.15 0.15 0.15 0.5] Grappled Reaction
  (Utilities|Time|ClearandInvalidateTimerbyHandle (Variables|Default|GetGrappledTimer))
  (Character|LaunchCharacter (Math|Vector|MakeVector (.x _returnvalue_6) 0.0 (+ (.z _returnvalue_6) 2.5e+02)) true true)
  (Variables|Default|Setgrappled false)
  (Variables|Default|SetStunned true)
  (Utilities|FlowControl|Delay 2.0)
  (Variables|Default|SetStunned false))

(event EventTick
  (params (DeltaSeconds :type Float%20%28single-precision%29))
  (bind _ceilingcheck (Variables|Default|GetCeilingCheck))
  (bind _linetracestartpoint (Variables|Default|GetLineTraceStartPoint))
  (bind _wallcheckdistance (Variables|Default|GetwallCheckDistance))
  (bind _returnvalue (Transformation|GetWorldLocation _ceilingcheck))
  (bind _returnvalue_2 (Transformation|GetWorldLocation _linetracestartpoint))
  (bind (_x _y _z) (Math|Vector|BreakVector _returnvalue_2))
  ;[0.15 0.15 0.15 0.5] Grapple stun (DONT MIND)
  (if (not (Variables|Default|GetStunned))
    (Utilities|FlowControl|Sequence
      (:then_0
        (if (Variables|Default|GetplayerDetected)
          (Utilities|FlowControl|Sequence
            (:then_0
              ;[0.15 0.15 0.15 0.5] Rotating the enemy based on it's moving direction
              (if (Variables|Default|GetDirection)
                (Transformation|SetActorRotation "0.000000,-90.000000,0.000000")
                (Development|PrintString "RIGHT")
                (else
                  (Transformation|SetActorRotation "0.000000,90.000000,0.000000")
                  (Development|PrintString "LEFT"))))
            (:then_1
              ;[0.15 0.15 0.15 0.5] Drawing line trace to detect walls
              (bind _outactors (Actor|GetAllActorswithInterface "/Game/Enemies/BPI_EnemyHealth.BPI_EnemyHealth_C"))
              (bind _returnvalue_3 (Collision|LineTraceByChannel _returnvalue_2 (Math|Vector|MakeVector (Math|Float|SelectFloat (+ _x _wallcheckdistance) (- _x _wallcheckdistance) (Variables|Default|GetDirection)) _y _z) "TraceTypeQuery1" false _outactors "ForOneFrame"))
              (if _returnvalue_3
                (if (Variables|Default|GethitWall)
                  (bind _returnvalue_4 (Collision|LineTraceByChannel _returnvalue (+ _returnvalue (* (Math|Vector|VectorUp) 35.0)) "TraceTypeQuery1" false 0 "ForOneFrame"))
                  (if _returnvalue_4
                    (Variables|Default|SetDirection (not (Variables|Default|GetDirection)))
                    (else
                      (Development|PrintString "CLIMBING")
                      (Variables|/Script/Engine.CharacterMovementComponent|SetGravityScale (Variables|Character|GetCharacterMovement) -0.5)
                      (Character|Jump)))
                  (else
                    ;[0.15 0.15 0.15 0.5] Climbing wall if wall was hit
                    (Variables|Default|SetplayerHit false)
                    (Variables|Default|SethitWall true)
                    (Variables|/Script/Engine.CharacterMovementComponent|SetGravityScale (Variables|Character|GetCharacterMovement) -0.5)
                    (Pawn|Input|AddMovementInput (Transformation|GetActorUpVector) 5.0 false)
                    (Character|Jump)
                    ;[0.15 0.15 0.15 0.5] Changing The Rotation Of The Spider's Mesh
                    (Transformation|SetWorldRotation (Variables|Collision|GetCapsuleComponent) "0.000000,-90.000000,0.000000" false false)))
                (else
                  ;[0.15 0.15 0.15 0.5] Not climbing wall is wall wasn't hit
                  (Variables|Default|SetplayerHit true)
                  (Variables|Default|SethitWall false)
                  (Variables|/Script/Engine.CharacterMovementComponent|SetGravityScale (Variables|Character|GetCharacterMovement) 1.0)))))))
      (:then_1
        ;[0.15 0.15 0.15 0.5] Rotating health text to face the camera
        (Transformation|SetWorldRotation (Variables|Default|GetHealthText) (Math|Rotator|MakeRotator 0.0 0.0 (.yaw (Math|Rotator|FindLookatRotation (Transformation|GetWorldLocation (Variables|Default|GetHealthText)) (Transformation|GetActorLocation (Game|GetPlayerCameraManager 0))))) false false)))))

(event EventBreakFreefromGrapple
  ;[0.15 0.15 0.15 0.5] Grappled Reaction
  (Variables|Default|Setgrappled false)
  (bind _asbp_2dcharacter (Utilities|Casting|CastToBP_2DCharacter (Game|GetPlayerCharacter 0)))
  (Default|RetractGrapple _asbp_2dcharacter))

(event EventEnemyDamage
  (params (Damage :type Integer))
  ;[0.15 0.15 0.15 0.5] Enemy damage. Called from the companion
  (Variables|Default|SetHealth (- (Variables|Default|GetHealth) Damage))
  ;[0.15 0.15 0.15 0.5] Health Check
  (if (<= (Variables|Default|GetHealth) 0)
    ;[0.15 0.15 0.15 0.5] Enemy Death
    (Actor|DestroyActor)
    (else
      ;[0.15 0.15 0.15 0.5] Updating Health Text if enemy isn't dead
      (Rendering|Components|TextRender|SetText (Variables|Default|GetHealthText) (Utilities|Text|ToText(Integer) (Variables|Default|GetHealth))))))

(event EventBeginPlay
  (bind _returnvalue (Transformation|GetActorLocation))
  ;[0.15 0.15 0.15 0.5] Correcting position on the Y axis
  (Transformation|SetActorLocation (Math|Vector|MakeVector (.x _returnvalue) (.y (Transformation|GetActorLocation (Game|Player|GetPlayerPawn 0))) (.z _returnvalue)) false true))

(fn ConstructionScript)