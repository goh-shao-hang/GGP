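; BP_Checkpoint is a checkpoint actor for a 2D game that heals the player and registers itself with the game mode.
; On BeginPlay it snaps its Y position to the player character's, and registers immediately if flagged as the default checkpoint.
; When a BP_2DCharacter overlaps it while inactive, it restores full health, stores itself in BP_2DGameMode, marks itself activated and prints a message.
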(event Custom|SetAsCheckpoint
  (bind _asbp_2dgame_mode (Utilities|Casting|CastToBP_2DGameMode (Game|GetGameMode)))
  (Variables|/Game/2D_Character/BP_2DGameMode.BP_2DGameMode_C|Setcheckpoint _asbp_2dgame_mode self)
  (Variables|Default|Setactivated true)
  (Development|PrintString "Reached checkpoint!"))

(event EventBeginPlay
  (bind _returnvalue (Transformation|GetActorLocation))
  (Transformation|SetActorLocation (Math|Vector|MakeVector (.x _returnvalue) (.y (Transformation|GetActorLocation (Game|GetPlayerCharacter 0))) (.z _returnvalue)) false false)
  (if (Variables|Default|GetisDefaultCheckpoint)
    (CallFunction|SetasCheckpoint)))

(event Collision|EventActorBeginOverlap
  (params (OtherActor :type Actor%20Object%20Reference))
  (if (not (Variables|Default|Getactivated))
    (bind _asbp_2dcharacter (Utilities|Casting|CastToBP_2DCharacter OtherActor))
    (Default|SettoFullHealth _asbp_2dcharacter)
    (CallFunction|SetasCheckpoint)))

(event EventTick
  (params (DeltaSeconds :type Float%20%28single-precision%29)))

(fn ConstructionScript)