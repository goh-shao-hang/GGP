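; A door Blueprint that opens once every lever in its Lever array is switched on.
; On BeginPlay it binds Check to each lever's true-state event, and Check rescans all lever states whenever one fires.
; When all are true, the TM_Move timeline lerps the stone door mesh's relative location from zero to TargetLocation.
; It has no logic for closing the door.
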(event Custom|Move
  (bind _lerp (Timeline|TM_Move Play)
    (:Update
      (Transformation|SetRelativeLocation (Variables|Default|Getstonedoor21) (Math|Vector|Lerp(Vector) "0, 0, 0" (Variables|Default|GettargetLocation) _lerp) false false))))

(event Custom|Check
  (Variables|Default|Setcompleted true)
  (for _array_element (Variables|Default|Getlever)
    (if (not (Variables|/Game/3D_Assets/BP_Lever.BP_Lever_C|GetleverState _array_element))
      (Variables|Default|Setcompleted false)))
  (if (Variables|Default|Getcompleted)
    (CallFunction|Move)))

(event EventBeginPlay
  (for _array_element (Variables|Default|Getlever)
    (EventDispatchers|BindEventtoOnTrueState _array_element (delegate Custom|Check))))

(fn ConstructionScript)