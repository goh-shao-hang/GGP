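; Toggleable lever actor that flips between two states when its pulled reaction event fires.
; On BeginPlay it moves itself to the player pawn's Y position, keeping its own X and Z.
; Each pull inverts LeverState, calls the OnTrueState or OnFalseState dispatcher, and plays or reverses a timeline that pitches the Pivot between its two angles.
; The Grapple event is an empty stub.
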(event EventBeginPlay
  (bind _returnvalue (Transformation|GetActorLocation))
  (Transformation|SetActorLocation (Math|Vector|MakeVector (.x _returnvalue) (.y (Transformation|GetActorLocation (Game|Player|GetPlayerPawn 0))) (.z _returnvalue)) false true))

(event Collision|EventActorBeginOverlap
  (params (OtherActor :type Actor%20Object%20Reference)))

(event EventTick
  (params (DeltaSeconds :type Float%20%28single-precision%29)))

(event EventGrapple)

(event EventPulledReaction
  (bind _output_get (Variables|Default|SetleverState (not (Variables|Default|GetleverState))))
  (if _output_get
    (Default|CallOnTrueState)
    (bind _lerp (Timeline|TM_LeverAnim Play)
      (:Update
        (Transformation|SetRelativeRotation (Variables|Default|GetPivot) (Math|Rotator|MakeRotator 0.0 (Math|Float|Lerp -4e+01 4e+01 _lerp) 0.0) false false)))
    (else
      (Default|CallOnFalseState)
      (Timeline|TM_LeverAnim Reverse))))

(fn ConstructionScript)